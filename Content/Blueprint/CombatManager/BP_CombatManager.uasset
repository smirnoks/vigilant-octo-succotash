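; BP_CombatManager limits how many attackers can attack a single AttackTarget at the same time.
; On BeginPlay it asks the target for its maximum attacker count through a message call.
; HandleAttackRequest ignores the target itself, then either adds the requester to Attackers and sends it an attack message, or adds it to WaitingAttack with a wait message.
; The file contains no logic for releasing slots or promoting waiting attackers.
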(event `self.ReceiveBeginPlay`
  (bind _value (message `/Game/Blueprint/CombatManager/BPI_AttackTarget.GetMaxAttackTarget` (`self.AttackTarget`)))
  (set `self.MaxAttackersCount` _value))

(fn `Handle Attack Request`
  (params (attacker :type "Actor Object Reference"))
  (bind _attacker (`local.attacker`))
  (bind _attacker_2 (`local.attacker`))
  (if (!= attacker (`self.AttackTarget`))
    (if (< (`KismetArrayLibrary.Array_Length` (`self.Attackers`)) (`self.MaxAttackersCount`))
      (`KismetArrayLibrary.Array_AddUnique` (`self.Attackers`) _attacker)
      (message `/Game/Blueprint/CombatManager/BPI_Attacker.Attack` _attacker (`self.AttackTarget`))
      (else
        (`KismetArrayLibrary.Array_AddUnique` (`self.WaitingAttack`) _attacker_2)
        (message `/Game/Blueprint/CombatManager/BPI_Attacker.Wait` _attacker_2 (`self.AttackTarget`))))))

(fn `UserConstructionScript`)